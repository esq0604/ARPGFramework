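; BP_Enemy is a katana-wielding enemy character that uses the Gameplay Ability System for attack and block.
; On BeginPlay it spawns a weapon actor, sets its trace channel responses, equips the katana data asset, grants both abilities and links the katana animation layer.
; The Dead event loosens mesh and capsule collision on pawn and custom trace channels, then sets it back after a fixed delay.
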(event `self.ReceiveBeginPlay`
  (bind _asc (`self.ASC`))
  (bind _returnvalue (`|SpawnActorFromClass` "/Game/Actor/BP_WeaponActor.BP_WeaponActor_C" (`self.GetTransform`) "Undefined" "MultiplyWithRoot" self self))
  (bind _output_get (set `self.WeaponInstance` _returnvalue))
  (`WeaponItem.SetTraceObjectType` _output_get "ECC_GameTraceChannel1" "ECR_Overlap")
  (`WeaponItem.SetTraceObjectType` _output_get "ECC_GameTraceChannel2" "ECR_Ignore")
  (`WeaponItem.EquipMesh` _output_get "/Game/Data/ItemData/PDA_Katana.PDA_Katana")
  (`AbilitySystemComponent.K2_GiveAbility` _asc "/Game/AbilitySystem/GameplayAbilities/GA_KatanaAttack.GA_KatanaAttack_C" 0 -1)
  (`AbilitySystemComponent.K2_GiveAbility` _asc "/Game/AbilitySystem/GameplayAbilities/GA_Block.GA_Block_C" 0 -1)
  (`SkeletalMeshComponent.LinkAnimClassLayers` (`self.Mesh`) "/Game/Animation/ALI_Katana_Anim_Layer.ALI_Katana_Anim_Layer_C"))

(event `self.Dead`
  (bind _mesh (`self.Mesh`))
  (bind _capsulecomponent (`self.CapsuleComponent`))
  (bind _capsulecomponent_2 (`self.CapsuleComponent`))
  (bind _mesh_2 (`self.Mesh`))
  (`PrimitiveComponent.SetCollisionResponseToChannel` _mesh_2 "ECC_Pawn" "ECR_Overlap")
  (`PrimitiveComponent.SetCollisionResponseToChannel` _mesh_2 "ECC_GameTraceChannel1" "ECR_Overlap")
  (`PrimitiveComponent.SetCollisionResponseToChannel` _capsulecomponent_2 "ECC_Pawn" "ECR_Overlap")
  (`PrimitiveComponent.SetCollisionResponseToChannel` _capsulecomponent_2 "ECC_GameTraceChannel1" "ECR_Overlap")
  (`PrimitiveComponent.SetCollisionResponseToChannel` _capsulecomponent_2 "ECC_GameTraceChannel3" "ECR_Ignore")
  (`KismetSystemLibrary.Delay` 4.0)
  (`PrimitiveComponent.SetCollisionResponseToChannel` _mesh "ECC_Pawn" "ECR_Block")
  (`PrimitiveComponent.SetCollisionResponseToChannel` _mesh "ECC_GameTraceChannel1" "ECR_Block")
  (`PrimitiveComponent.SetCollisionResponseToChannel` _capsulecomponent "ECC_Pawn" "ECR_Block")
  (`PrimitiveComponent.SetCollisionResponseToChannel` _capsulecomponent "ECC_GameTraceChannel1" "ECR_Block")
  (`PrimitiveComponent.SetCollisionResponseToChannel` _capsulecomponent "ECC_GameTraceChannel3" "ECR_Overlap"))

(fn `UserConstructionScript`)