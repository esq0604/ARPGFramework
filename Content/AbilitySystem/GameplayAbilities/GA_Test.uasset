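; Test Gameplay Ability that runs a melee combo, playing the attack montage for the current index in NewVar's ComboInfos.
; While the CanNextAttack tag is present, an input press advances the index and plays the next montage, and tag removal closes that window.
; Montage completion or blend-out ends the ability and resets the combo, as does a hard-coded stop at index 3; interruption cancels it.
; Hit handling is an unconnected stub.
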(event `self.K2_ActivateAbility`
  (bind (_returnvalue_owneractor _returnvalue_avataractor) (break `GameplayAbilityActorInfo` (`self.GetActorInfo`)))
  (bind _intputtask (`self.IntputTask`))
  (bind _addedtagtask (`self.AddedTagTask`))
  (bind _addedtagtask_2 (`self.AddedTagTask`))
  (bind _removetagtask (`self.RemoveTagTask`))
  (bind _comboinfos (`ComboDataAsset.ComboInfos` (`self.NewVar`)))
  (bind (_attackmontage _deflectedmontage _hitreactioninfos) (break `ComboInfo` (`|GetArrayItem` _comboinfos (`self.CurrentComboIndex`))))
  (`self.K2_CommitAbility`)
  (if (== (`self.CurrentComboIndex`) 3) :!label _label
    (`self.K2_EndAbility`)
    (elif (not (== (`KismetArrayLibrary.Array_Length` _comboinfos) 0))
      (`AbilityTask_PlayMontageAndWait.CreatePlayMontageAndWaitProxy` "None" _attackmontage
        (:`then`
          (for _ _hitreactioninfos
            _)
          (bind _asynctaskproxy (`AbilityTask_WaitGameplayTagAdded.WaitGameplayTagAdd` (struct :`TagName` "State.Attack.CanNextAttack") null)
            (:`then`
              (set `self.AddedTagTask` _asynctaskproxy))
            (:`Added`
              (bind _asynctaskproxy_2 (`AbilityTask_WaitInputPress.WaitInputPress` false)
                (:`then`
                  (set `self.IntputTask` _asynctaskproxy_2)
                  (bind _asynctaskproxy_3 (`AbilityTask_WaitGameplayTagRemoved.WaitGameplayTagRemove` (struct :`TagName` "State.Attack.CanNextAttack") null)
                    (:`then`
                      (set `self.RemoveTagTask` _asynctaskproxy_3))
                    (:`Removed`
                      (if (`KismetSystemLibrary.IsValid` _intputtask)
                        (`GameplayTask.EndTask` _intputtask)
                        (if (`KismetSystemLibrary.IsValid` _addedtagtask)
                          (`GameplayTask.EndTask` _addedtagtask))))))
                (:`OnPress`
                  (if (`KismetSystemLibrary.IsValid` _addedtagtask_2)
                    (`GameplayTask.EndTask` _addedtagtask_2)
                    (if (`KismetSystemLibrary.IsValid` _removetagtask)
                      (`GameplayTask.EndTask` _removetagtask)
                      (bind _result (`/Engine/EditorBlueprintResources/StandardMacros.IncrementInt` (`self.CurrentComboIndex`))
                        (:`  `
                          (bind _output_get (set `self.CurrentComboIndex` (mod _result (`KismetArrayLibrary.Array_Length` (`ComboDataAsset.ComboInfos` (`self.NewVar`))))))
                          (`KismetSystemLibrary.PrintString` (`KismetStringLibrary.Concat_StrStr` "cur Combo Index" (`KismetStringLibrary.Conv_IntToString` _output_get)))
                          (goto _label))))))))))
        (:`OnCompleted`
          (`self.K2_EndAbility` :!label _label_2))
        (:`OnBlendOut`
          (goto _label_2))
        (:`OnInterrupted`
          (`AbilitySystemBlueprintLibrary.RemoveLooseGameplayTags` _returnvalue_avataractor (`BlueprintGameplayTagLibrary.MakeLiteralGameplayTagContainer` (struct :`GameplayTags` (struct :`(TagName` "State.Attack.CanNextAttack")))))
          (`self.K2_CancelAbility` :!label _label_3))
        (:`OnCancelled`
          (goto _label_3))))))

(event `self.K2_OnEndAbility`
  (params (bWasCancelled :type Boolean))
  (if bWasCancelled
    (`KismetSystemLibrary.PrintString` "cancel ability")
    (else
      (`KismetSystemLibrary.PrintString` "end ability")
      (set `self.CurrentComboIndex` 0))))

(fn `AttackAtive`)

(fn `AttackHit`)