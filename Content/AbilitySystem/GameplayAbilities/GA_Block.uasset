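; GA_Block is a hold-to-block gameplay ability.
; On activation it commits, adds animation tags to the avatar and applies GE_Block, then removes the tags and ends on input release.
; It also listens for State.Attack effects blocked by immunity; when GE_Block is the blocker, it executes the GameplayCue.Block cue with the attacker's context and prints the instigator's name.
; A comment notes that directional blocking is required, but no direction check exists.
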(event `self.K2_ActivateAbility`
  ;[1 1 1] 방향에따라 방어해야합니다
  (bind _returnvalue (`self.K2_CommitAbility`))
  (if _returnvalue
    (`|ExecutionSequence`
      (:`then_0`
        (`AbilitySystemBlueprintLibrary.AddLooseGameplayTags` (`self.GetAvatarActorFromActorInfo`) (`self.AnimationTag`))
        (`AbilityTask_WaitInputRelease.WaitInputRelease` false
          (:`OnRelease`
            (`AbilitySystemBlueprintLibrary.RemoveLooseGameplayTags` (`self.GetAvatarActorFromActorInfo`) (`self.AnimationTag`))
            (`self.K2_EndAbility`))))
      (:`then_1`
        (bind _returnvalue_2 (`self.BP_ApplyGameplayEffectToOwner` "/Game/AbilitySystem/GameplayEffects/GE_Block.GE_Block_C"))
        (set `self.BlcokEffectHandle` _returnvalue_2))
      (:`then_2`
        (bind (_asynctaskproxy _blockedspec _immunitygameplayeffecthandle) (`AbilityTask_WaitGameplayEffectBlockedImmunity.WaitGameplayEffectBlockedByImmunity` (make `GameplayTagRequirements` (struct :`GameplayTags` (struct :`(TagName` "State.Attack")))) (struct) null)
          (:`Blocked`
            (bind _returnvalue_3 (`AbilitySystemBlueprintLibrary.GetEffectContext` _blockedspec))
            (if (== (`GameplayStatics.GetObjectClass` (`AbilitySystemBlueprintLibrary.GetGameplayEffectFromActiveEffectHandle` _immunitygameplayeffecthandle)) "/Game/AbilitySystem/GameplayEffects/GE_Block.GE_Block_C")
              (`GameplayCueFunctionLibrary.ExecuteGameplayCueOnActor` (`self.GetAvatarActorFromActorInfo`) (struct :`TagName` "GameplayCue.Block") (`AbilitySystemBlueprintLibrary.MakeGameplayCueParameters` 0.0 0.0 _returnvalue_3 (struct) (struct) (struct) (struct) (0.0 0.0 0.0) (0.0 0.0 0.0) (`AbilitySystemBlueprintLibrary.EffectContextGetInstigatorActor` _returnvalue_3)))
              (`KismetSystemLibrary.PrintString` (`KismetSystemLibrary.GetDisplayName` (`AbilitySystemBlueprintLibrary.EffectContextGetInstigatorActor` _returnvalue_3))))))))))

(event `self.K2_OnEndAbility`
  (params (bWasCancelled :type Boolean))
  (bind (_returnvalue_owneractor _returnvalue_avataractor) (break `GameplayAbilityActorInfo` (`self.GetActorInfo`)))
  ;[1 1 1] 방향에따라 방어해야합니다
  (`AbilitySystemBlueprintLibrary.RemoveLooseGameplayTags` _returnvalue_avataractor (`self.AnimationTag`)))

(fn `IsBlockSuccced`
  (params (NewParam :type "HitResult Structure")))